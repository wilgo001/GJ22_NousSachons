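; Portal actor that shows the view from its ConnectedPortal and teleports the player to it.
; On BeginPlay the linked portal's scene capture feeds a new render target shown through a dynamic material on the plane; the capture is not moved here.
; Plane overlap offsets the player between arrows, applies their yaw difference and reassigns unrotated velocity.
; CanTP gates teleporting, toggled by the in/out cap overlaps and cleared on the destination.
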(event OnComponentBeginOverlap(SM_Plane)
  (params (OverlappedComponent :type Primitive%20Component%20Object%20Reference) (OtherActor :type Actor%20Object%20Reference) (OtherComp :type Primitive%20Component%20Object%20Reference) (OtherBodyIndex :type Integer) (bFromSweep :type Boolean) (SweepResult :type Hit%20Result%20Structure%20%28by%20ref%29))
  (bind _returnvalue (Game|GetPlayerController 0))
  (bind _returnvalue_2 (Game|GetPlayerCharacter 0))
  (bind _returnvalue_3 (Transformation|GetActorRotation _returnvalue))
  (if (== OtherActor _returnvalue_2)
    (if (Variables|Default|GetcanTP)
      (Variables|/Game/Portal_New/BP_Portal2.BP_Portal2_C|SetcanTP (Variables|Default|GetConnectedPortal) false)
      (Transformation|SetActorLocation _returnvalue_2 (+ (- (Transformation|GetWorldLocation (Variables|Default|GetArrowIn)) (Transformation|GetActorLocation _returnvalue_2)) (Transformation|GetWorldLocation (Variables|/Game/Portal_New/BP_Portal2.BP_Portal2_C|GetArrowOut (Variables|Default|GetConnectedPortal)))) false false)
      (Pawn|SetControlRotation (Game|GetPlayerController 0) (Math|Rotator|MakeRotator (.roll _returnvalue_3) (.pitch _returnvalue_3) (+ (- (.yaw (Transformation|GetWorldRotation (Variables|/Game/Portal_New/BP_Portal2.BP_Portal2_C|GetArrowOut (Variables|Default|GetConnectedPortal)))) (.yaw (Transformation|GetWorldRotation (Variables|Default|GetArrowIn)))) (.yaw _returnvalue_3))))
      (Variables|/Script/Engine.MovementComponent|SetVelocity (Variables|/Script/Engine.Character|GetCharacterMovement (Game|GetPlayerCharacter 0)) (Transformation|GetVelocity _returnvalue_2)))))

(event OnComponentBeginOverlap(InCaps)
  (params (OverlappedComponent :type Primitive%20Component%20Object%20Reference) (OtherActor :type Actor%20Object%20Reference) (OtherComp :type Primitive%20Component%20Object%20Reference) (OtherBodyIndex :type Integer) (bFromSweep :type Boolean) (SweepResult :type Hit%20Result%20Structure%20%28by%20ref%29))
  (bind _output_get (Variables|Default|SetcanTP (== OtherActor (Game|GetPlayerCharacter 0))))
  (Development|PrintText (Utilities|Text|ToText(Boolean) _output_get)))

(event OnComponentBeginOverlap(OutCaps)
  (params (OverlappedComponent :type Primitive%20Component%20Object%20Reference) (OtherActor :type Actor%20Object%20Reference) (OtherComp :type Primitive%20Component%20Object%20Reference) (OtherBodyIndex :type Integer) (bFromSweep :type Boolean) (SweepResult :type Hit%20Result%20Structure%20%28by%20ref%29))
  (if (== OtherActor (Game|GetPlayerCharacter 0))
    (bind _output_get (Variables|Default|SetcanTP false))
    (Development|PrintText (Utilities|Text|ToText(Boolean) _output_get))))

(event EventBeginPlay
  ;[1 1 1] setup material plane
  (bind _returnvalue (Rendering|Material|CreateDynamicMaterialInstance (Variables|Default|GetSM_Plane) 0 "/Game/Portal_New/MA_Portal2.MA_Portal2" "None" :!class /Script/Engine.PrimitiveComponent))
  (bind _returnvalue_2 (Rendering|CreateRenderTarget2D 1920 1080 "RTF_RGBA16f"))
  (bind _output_get (Variables|/Script/Engine.SceneCaptureComponent2D|SetTextureTarget (Variables|/Game/Portal_New/BP_Portal2.BP_Portal2_C|GetSC_Capture (Variables|Default|GetConnectedPortal)) _returnvalue_2))
  (Rendering|Material|SetTextureParameterValue _returnvalue "Color" _output_get))

(event EventTick
  (params (DeltaSeconds :type Float%20%28single-precision%29)))

(fn ConstructionScript
  (Variables|Default|SetcanTP true))