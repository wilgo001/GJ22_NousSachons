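; Portal manager that keeps the view through a linked pair of portals, Portal1 and Portal2, in step with the player's camera.
; Every Tick, two mirrored update functions each move one portal's SCCapture component to the player camera's pose remapped from the other portal's frame.
; The remap uses the rotation delta between the portal roots, with a 180-degree yaw flip on the destination, to transform both camera location and rotation.
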(event EventBeginPlay)

(event Collision|EventActorBeginOverlap
  (params (OtherActor :type Actor%20Object%20Reference)))

(event EventTick
  (params (DeltaSeconds :type Float%20%28single-precision%29))
  (CallFunction|Portal1Update)
  (CallFunction|Portal2Update))

(fn ConstructionScript)

(fn Portal1Update
  (bind _returnvalue (Game|GetPlayerController 0))
  (bind _portal1 (Variables|Default|Getportal1))
  (bind _portal2 (Variables|Default|Getportal2))
  (bind _defaultsceneroot (Variables|/Game/Portal/BP_Portal1.BP_Portal1_C|GetDefaultSceneRoot _portal1))
  (bind _defaultsceneroot_2 (Variables|/Game/Portal/BP_Portal2.BP_Portal2_C|GetDefaultSceneRoot _portal2))
  (bind _playercameramanager (Variables|/Script/Engine.PlayerController|GetPlayerCameraManager _returnvalue))
  (bind _returnvalue_2 (Transformation|GetWorldRotation _defaultsceneroot_2))
  (bind _returnvalue_3 (Transformation|GetWorldRotation _defaultsceneroot))
  (bind _transformcomponent (Variables|/Script/Engine.PlayerCameraManager|GetTransformComponent _playercameramanager))
  (bind _returnvalue_4 (- (.yaw _returnvalue_2) 1.8e+02))
  (bind _returnvalue_5 (Math|Rotator|MakeRotator (.roll _returnvalue_2) (.pitch _returnvalue_2) _returnvalue_4))
  (bind _returnvalue_6 (Math|Rotator|Delta(Rotator) _returnvalue_5 _returnvalue_3))
  (Transformation|SetWorldLocationAndRotation (Variables|/Game/Portal/BP_Portal2.BP_Portal2_C|GetSC_Capture (Variables|Default|Getportal2)) (+ (- (Transformation|GetWorldLocation _defaultsceneroot_2) (Math|Vector|RotateVector (Transformation|GetWorldLocation _defaultsceneroot) _returnvalue_6)) (Math|Vector|RotateVector (Transformation|GetWorldLocation _transformcomponent) _returnvalue_6)) (Math|Rotator|CombineRotators (Transformation|GetWorldRotation _transformcomponent) _returnvalue_6) false false))

(fn Portal2Update
  (bind _returnvalue (Game|GetPlayerController 0))
  (bind _portal1 (Variables|Default|Getportal1))
  (bind _portal2 (Variables|Default|Getportal2))
  (bind _defaultsceneroot (Variables|/Game/Portal/BP_Portal1.BP_Portal1_C|GetDefaultSceneRoot _portal1))
  (bind _defaultsceneroot_2 (Variables|/Game/Portal/BP_Portal2.BP_Portal2_C|GetDefaultSceneRoot _portal2))
  (bind _playercameramanager (Variables|/Script/Engine.PlayerController|GetPlayerCameraManager _returnvalue))
  (bind _returnvalue_2 (Transformation|GetWorldRotation _defaultsceneroot))
  (bind _returnvalue_3 (Transformation|GetWorldRotation _defaultsceneroot_2))
  (bind _transformcomponent (Variables|/Script/Engine.PlayerCameraManager|GetTransformComponent _playercameramanager))
  (bind _returnvalue_4 (- (.yaw _returnvalue_2) 1.8e+02))
  (bind _returnvalue_5 (Math|Rotator|MakeRotator (.roll _returnvalue_2) (.pitch _returnvalue_2) _returnvalue_4))
  (bind _returnvalue_6 (Math|Rotator|Delta(Rotator) _returnvalue_5 _returnvalue_3))
  (Transformation|SetWorldLocationAndRotation (Variables|/Game/Portal/BP_Portal1.BP_Portal1_C|GetSC_Capture (Variables|Default|Getportal1)) (+ (- (Transformation|GetWorldLocation _defaultsceneroot) (Math|Vector|RotateVector (Transformation|GetWorldLocation _defaultsceneroot_2) _returnvalue_6)) (Math|Vector|RotateVector (Transformation|GetWorldLocation _transformcomponent) _returnvalue_6)) (Math|Rotator|CombineRotators (Transformation|GetWorldRotation _transformcomponent) _returnvalue_6) false false))