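; Portal actor that shows the view from a linked portal and teleports the player to it.
; On BeginPlay, the linked portal's scene capture gets a render target that feeds this plane's dynamic material.
; InCaps and OutCaps overlaps toggle and print CanTP, which gates EnterPortal.
; Teleporting disables the linked portal's CanTP, offsets the player using both arrows, adjusts control yaw by their difference and reapplies velocity unrotated.
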(event OnComponentBeginOverlap(enterPortal)
  (params (OverlappedComponent :type Primitive%20Component%20Object%20Reference) (OtherActor :type Actor%20Object%20Reference) (OtherComp :type Primitive%20Component%20Object%20Reference) (OtherBodyIndex :type Integer) (bFromSweep :type Boolean) (SweepResult :type Hit%20Result%20Structure%20%28by%20ref%29))
  (bind _returnvalue (Game|GetPlayerCharacter 0))
  (bind _returnvalue_2 (Game|GetPlayerController 0))
  (bind _rootcomponent (Variables|/Script/Engine.Actor|GetRootComponent _returnvalue_2))
  (bind _returnvalue_3 (Transformation|GetWorldRotation _rootcomponent))
  (if (== OtherActor _returnvalue)
    (if (Variables|Default|GetcanTP)
      (Variables|/Game/Portal/BP_Portal1.BP_Portal1_C|SetcanTP (Variables|Default|GetconnectdPortal) false)
      (Transformation|SetActorLocation _returnvalue (+ (- (Transformation|GetWorldLocation (Variables|Default|GetArrowIn)) (Transformation|GetActorLocation _returnvalue)) (Transformation|GetWorldLocation (Variables|/Game/Portal/BP_Portal1.BP_Portal1_C|GetArrowOut (Variables|Default|GetconnectdPortal)))) false false)
      (Pawn|SetControlRotation (Game|GetPlayerController 0) (Math|Rotator|MakeRotator (.roll _returnvalue_3) (.pitch _returnvalue_3) (+ (- (.yaw (Transformation|GetWorldRotation (Variables|/Game/Portal/BP_Portal1.BP_Portal1_C|GetArrowOut (Variables|Default|GetconnectdPortal)))) (.yaw (Transformation|GetWorldRotation (Variables|Default|GetArrowIn)))) (.yaw _returnvalue_3))))
      (Variables|/Script/Engine.MovementComponent|SetVelocity (Variables|/Script/Engine.Character|GetCharacterMovement (Game|GetPlayerCharacter 0)) (Transformation|GetVelocity _returnvalue)))))

(event OnComponentBeginOverlap(OutCaps)
  (params (OverlappedComponent :type Primitive%20Component%20Object%20Reference) (OtherActor :type Actor%20Object%20Reference) (OtherComp :type Primitive%20Component%20Object%20Reference) (OtherBodyIndex :type Integer) (bFromSweep :type Boolean) (SweepResult :type Hit%20Result%20Structure%20%28by%20ref%29))
  (if (== OtherActor (Game|GetPlayerCharacter 0))
    (bind _output_get (Variables|Default|SetcanTP false))
    (Development|PrintText (Utilities|Text|ToText(Boolean) _output_get))))

(event OnComponentBeginOverlap(InCaps)
  (params (OverlappedComponent :type Primitive%20Component%20Object%20Reference) (OtherActor :type Actor%20Object%20Reference) (OtherComp :type Primitive%20Component%20Object%20Reference) (OtherBodyIndex :type Integer) (bFromSweep :type Boolean) (SweepResult :type Hit%20Result%20Structure%20%28by%20ref%29))
  (bind _output_get (Variables|Default|SetcanTP (== OtherActor (Game|GetPlayerCharacter 0))))
  (Development|PrintText (Utilities|Text|ToText(Boolean) _output_get)))

(event EventBeginPlay
  (bind _returnvalue (Rendering|Material|CreateDynamicMaterialInstance (Variables|Default|GetSM_Plane) 0 "/Game/Portal/MA_Portal2.MA_Portal2" "None" :!class /Script/Engine.PrimitiveComponent))
  (bind _returnvalue_2 (Rendering|CreateRenderTarget2D 1920 1080 "RTF_RGBA16f"))
  (bind _output_get (Variables|/Script/Engine.SceneCaptureComponent2D|SetTextureTarget (Variables|/Game/Portal/BP_Portal1.BP_Portal1_C|GetSC_Capture (Variables|Default|GetconnectdPortal)) _returnvalue_2))
  (Rendering|Material|SetTextureParameterValue _returnvalue "Color" _output_get))

(event EventTick
  (params (DeltaSeconds :type Float%20%28single-precision%29)))

(fn ConstructionScript
  (Variables|Default|SetcanTP true))