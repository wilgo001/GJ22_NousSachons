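; Pushable box that the player moves onto a BP_PressurePlate, respawning at its start location if not placed in time.
; Player overlap with X_Box or Y_Box enables physics and, on first contact since spawning, starts a RespawnDuration delay before teleporting back unless plated.
; Overlapping a free plate snaps the box to its Plane, marks the plate occupied and disables physics, locking the box there.
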(event OnComponentBeginOverlap(X_Box)
  (params (OverlappedComponent :type Primitive%20Component%20Object%20Reference) (OtherActor :type Actor%20Object%20Reference) (OtherComp :type Primitive%20Component%20Object%20Reference) (OtherBodyIndex :type Integer) (bFromSweep :type Boolean) (SweepResult :type Hit%20Result%20Structure%20%28by%20ref%29))
  (if (== OtherActor (Game|GetPlayerCharacter 0))
    (if (not (Variables|Default|GetisOnPlane))
      (Physics|SetSimulatePhysics (Variables|Default|GetBox) true)
      (CallFunction|CheckifonSpawn))))

(event OnComponentBeginOverlap(Y_Box)
  (params (OverlappedComponent :type Primitive%20Component%20Object%20Reference) (OtherActor :type Actor%20Object%20Reference) (OtherComp :type Primitive%20Component%20Object%20Reference) (OtherBodyIndex :type Integer) (bFromSweep :type Boolean) (SweepResult :type Hit%20Result%20Structure%20%28by%20ref%29))
  (if (== OtherActor (Game|GetPlayerCharacter 0))
    (if (not (Variables|Default|GetisOnPlane))
      (Physics|SetSimulatePhysics (Variables|Default|GetBox) true)
      (CallFunction|CheckifonSpawn))))

(event OnComponentEndOverlap(X_Box)
  (params (OverlappedComponent :type Primitive%20Component%20Object%20Reference) (OtherActor :type Actor%20Object%20Reference) (OtherComp :type Primitive%20Component%20Object%20Reference) (OtherBodyIndex :type Integer)))

(event OnComponentEndOverlap(Y_Box)
  (params (OverlappedComponent :type Primitive%20Component%20Object%20Reference) (OtherActor :type Actor%20Object%20Reference) (OtherComp :type Primitive%20Component%20Object%20Reference) (OtherBodyIndex :type Integer)))

(event OnComponentBeginOverlap(Box)
  (params (OverlappedComponent :type Primitive%20Component%20Object%20Reference) (OtherActor :type Actor%20Object%20Reference) (OtherComp :type Primitive%20Component%20Object%20Reference) (OtherBodyIndex :type Integer) (bFromSweep :type Boolean) (SweepResult :type Hit%20Result%20Structure%20%28by%20ref%29))
  (bind _asbp_pressure_plate (Utilities|Casting|CastToBP_PressurePlate OtherActor))
  (if (not (Variables|/Game/PressurePlate/BP_PressurePlate.BP_PressurePlate_C|GetalreadyHaveBox _asbp_pressure_plate))
    (Variables|/Game/PressurePlate/BP_PressurePlate.BP_PressurePlate_C|SetalreadyHaveBox _asbp_pressure_plate true)
    (Transformation|SetWorldLocation (Variables|Default|GetBox) (Transformation|GetWorldLocation (Variables|/Game/PressurePlate/BP_PressurePlate.BP_PressurePlate_C|GetPlane _asbp_pressure_plate)) false true)
    (Variables|Default|SetisOnPlane true)
    (Physics|SetSimulatePhysics (Variables|Default|GetBox) false)))

(event Custom|CheckIfOnSpawn
  (if (Variables|Default|GetisOnSpawn)
    (Variables|Default|SetisOnSpawn false)
    (Utilities|FlowControl|Delay (Variables|Default|GetrespawnDuration))
    (if (not (Variables|Default|GetisOnPlane))
      (CallFunction|ResetonSpawn))))

(event Custom|ResetOnSpawn
  (Transformation|SetWorldLocation (Variables|Default|GetBox) (Variables|Default|GetSpawnLocation) false true)
  (Variables|Default|SetisOnSpawn true))

(event EventBeginPlay
  (Variables|Default|SetSpawnLocation (Transformation|GetWorldLocation (Variables|Default|GetBox)))
  (Variables|Default|SetisOnSpawn true)
  (Variables|Default|SetisOnPlane false))

(fn ConstructionScript
  (Variables|Default|SetisOnSpawn true)
  (Variables|Default|SetSpawnLocation (Transformation|GetWorldLocation (Variables|Default|GetDefaultSceneRoot)))
  (Variables|Default|SetcanTP false))